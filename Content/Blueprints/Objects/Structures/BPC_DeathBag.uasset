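; Death bag actor, a lootable container that holds the items passed to it in DeathInventory.
; The construction script counts non-empty entries to size the inventory and copies the array into its inventory component, destroying the actor if none exist.
; Interacting opens the container on the FPS HUD, and cursor hover reports to the top-down HUD.
; When an inventory update leaves it empty, it removes the menu and destroys itself.
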(event `self.InteractWith`
  (params (PlayerCharacter :type "/Game/Blueprints/Player/BP_CharacterParent Object Reference"))
  (`/Game/Blueprints/UI/WB_FPS_Hud.ShowContainer` (`/Game/Blueprints/Framework/BP_PlayerController.Ref_FPS_HUD` (`/Game/Blueprints/Framework/BFL_GeneralUse.CastToPlayerController`)) (`self.BPAC_InventorySystem`)))

(event `self.ReceiveActorBeginCursorOver`
  (`/Game/Blueprints/UI/WB_TD_Hud.HoveredObjectUpdate` (`/Game/Blueprints/Framework/BP_PlayerController.Ref_TD_Hud` (`/Game/Blueprints/Framework/BFL_GeneralUse.CastToPlayerController`)) true self "None"))

(event `self.ReceiveActorEndCursorOver`
  (`/Game/Blueprints/UI/WB_TD_Hud.HoveredObjectUpdate` (`/Game/Blueprints/Framework/BP_PlayerController.Ref_TD_Hud` (`/Game/Blueprints/Framework/BFL_GeneralUse.CastToPlayerController`)) false self "None"))

(event `self.BPAC_InventorySystem.InventoryUpdated`
  (if (<= (`/Game/Blueprints/Framework/Component/BPAC_InventorySystem.GetQuantity` (`self.BPAC_InventorySystem`)) 0)
    (`Widget.RemoveFromParent` (`/Game/Blueprints/UI/WB_FPS_Hud.Ref_Menu` (`/Game/Blueprints/Framework/BP_PlayerController.Ref_FPS_HUD` (`/Game/Blueprints/Framework/BFL_GeneralUse.CastToPlayerController`))))
    (`self.K2_DestroyActor`)))

(fn `UserConstructionScript`
  (locals (Lcl_InventoryAmount :type Integer))
  (bind _deathinventory (`self.DeathInventory`))
  (bind _lcl_inventoryamount (`local.Lcl_InventoryAmount`))
  (`parent.UserConstructionScript`)
  (for _array_element _deathinventory
    (if (!= (`.ItemID_2_7E5047D54E17F2E220EDF586F14F2261` (break `/Game/Blueprints/Framework/Structs/S_InventorySlots` _array_element)) "None")
      (`/Engine/EditorBlueprintResources/StandardMacros.IncrementInt` (`local.Lcl_InventoryAmount`))))
  (if (>= _lcl_inventoryamount 1)
    (set `self.InventorySize` _lcl_inventoryamount)
    (set `/Game/Blueprints/Framework/Component/BPAC_InventorySystem.Content` _deathinventory (`self.BPAC_InventorySystem`))
    (else
      (`self.K2_DestroyActor`))))