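; Parent character Blueprint for units that are hovered, selected and moved in top-down view, with mesh swapping for first-person possession.
; Construction loads name, note and gameplay tags from DT_CharacterInfo, choosing the selection decal by tag.
; Cursor events update the HUD and player controller selection; unpossessing toggles meshes and selection, restarting AI when leaving player control.
; A looping delay drains Food, whose OnRep writes hunger to the AI blackboard.
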(event `self.ReceiveActorBeginCursorOver`
  ;[1 1 1] Hovered
  (`/Game/Blueprints/UI/WB_TD_Hud.HoveredObjectUpdate` (`/Game/Blueprints/Framework/BP_PlayerController.Ref_TD_Hud` (`/Game/Blueprints/Framework/BFL_GeneralUse.CastToPlayerController`)) true self (`self.RowID`)))

(event `self.ReceiveTick`
  (params (DeltaSeconds :type "Float (single-precision)"))
  ;[1 0 0] Event Tick
)

(event `self.ReceiveActorEndCursorOver`
  ;[1 1 1] Hovered
  (`/Game/Blueprints/UI/WB_TD_Hud.HoveredObjectUpdate` (`/Game/Blueprints/Framework/BP_PlayerController.Ref_TD_Hud` (`/Game/Blueprints/Framework/BFL_GeneralUse.CastToPlayerController`)) false self "None"))

(event `Moving`
  (params (Goal :type "Vector Structure (by ref)"))
  (bind _aicontroller (`self.AIController`))
  ;[1 1 1] Unit Moving
  (`Controller.StopMovement` _aicontroller)
  (`AIBlueprintHelperLibrary.SimpleMoveToLocation` _aicontroller Goal))

(event `self.ReceiveBeginPlay`
  ;[1 1 1] Begin Play
  (`self.SetAIController`)
  (set `self.AIBlackBoard` (`AIBlueprintHelperLibrary.GetBlackboard` null))
  (`self.Hunger`))

(event `Hunger`
  ;[1 1 1] Unit Hunger Stat
  (if (>= (`self.Food`) 0) :!label _label
    (set `self.Food` (- (`self.Food`) 25))
    (`KismetSystemLibrary.Delay` 1.0)
    (goto _label)
    (else
      (`KismetSystemLibrary.PrintString` (`KismetTextLibrary.Conv_TextToString` (`|FormatText` "Starving \n \n--BP_FPSPlayerCharacter--")) true true (struct :`R` 1.0 :`A` 1.0)))))

(event `self.ReceiveActorOnClicked`
  (params (ButtonPressed :type "Key Structure"))
  (bind _asbp_player_controller (`/Game/Blueprints/Framework/BFL_GeneralUse.CastToPlayerController`))
  (bind _currentselectedcharacter (`/Game/Blueprints/Framework/BP_PlayerController.CurrentSelectedCharacter` _asbp_player_controller))
  ;[1 1 1] When Unit is selected
  (`/Engine/EditorBlueprintResources/StandardMacros.IsValid` _currentselectedcharacter
    (:`Is Valid`
      (`self.DeselectedCharacter` _currentselectedcharacter))
    (:`Is Not Valid`
      _))
  (set `/Game/Blueprints/Framework/BP_PlayerController.CurrentSelectedCharacter` self _asbp_player_controller)
  (`/Game/Blueprints/Framework/BP_PlayerController.EnableControls` _asbp_player_controller true false false)
  (`self.SelectedCharacter`))

(event `self.ReceiveUnpossessed`
  (params (OldController :type "Controller Object Reference"))
  ;[1 1 1] Unpossessed
  (if (== OldController (`self.AIController`))
    (`SceneComponent.SetHiddenInGame` (`self.Mesh`) true false)
    (`SceneComponent.SetHiddenInGame` (`self.FirstPersonMesh`) false false)
    (`self.DeselectedCharacter`)
    (else
      (`SceneComponent.SetHiddenInGame` (`self.Mesh`) false false)
      (`SceneComponent.SetHiddenInGame` (`self.FirstPersonMesh`) true false)
      (`self.SelectedCharacter`)
      (`self.SetAIController`))))

(event `SelectedCharacter`
  ;[1 1 1] Adding Decal
  (`SceneComponent.SetVisibility` (`self.SelectionDecal`) true false)
  (set `self.IsSelected` true)
  (`/Game/Blueprints/UI/WB_TD_Hud.SelectedCharacter` (`/Game/Blueprints/Framework/BP_PlayerController.Ref_TD_Hud` (`/Game/Blueprints/Framework/BFL_GeneralUse.CastToPlayerController`)) true (`self.RowID`)))

(event `DeselectedCharacter`
  ;[1 1 1] Adding Decal
  (`SceneComponent.SetVisibility` (`self.SelectionDecal`) false false)
  (set `self.IsSelected` false))

(fn `GetGameplayTags`
  (returns (Tags :type "GameplayTagContainer Structure"))
  (return (`self.GameplayTags`)))

(fn `OnRep_Food`
  (`BlackboardComponent.SetValueAsInt` (`self.AIBlackBoard`) "UnitHunger" (`self.Food`)))

(fn `SetAIController`
  (`/Engine/EditorBlueprintResources/StandardMacros.IsValid` (`self.AIController`)
    (:`Is Valid`
      _)
    (:`Is Not Valid`
      (bind _asbp_aiplayer_units (cast `/Game/Blueprints/AI/BP_AIPlayerUnits` (`AIBlueprintHelperLibrary.GetAIController` self)))
      (set `self.AIController` _asbp_aiplayer_units)))
  (`/Game/Blueprints/AI/BP_AIPlayerUnits.RunAI` (`self.AIController`))
  (return))

(fn `SetSelectedDecal`
  (bind _gameplaytags (`self.GameplayTags`))
  (bind _selectiondecal (`self.SelectionDecal`))
  (if (`BlueprintGameplayTagLibrary.HasTag` _gameplaytags (struct :`TagName` "People.Recruited"))
    (`DecalComponent.SetDecalMaterial` _selectiondecal "/Game/Art/Decals/M_SelectedRecruitedDecal.M_SelectedRecruitedDecal")
    (elif (`BlueprintGameplayTagLibrary.HasTag` _gameplaytags (struct :`TagName` "People.Recruitable"))
      (`DecalComponent.SetDecalMaterial` _selectiondecal "/Game/Art/Decals/M_SelectedNonRecruitedDecal.M_SelectedNonRecruitedDecal")
      (elif (`BlueprintGameplayTagLibrary.HasTag` _gameplaytags (struct :`TagName` "People.Evil"))
        (`DecalComponent.SetDecalMaterial` _selectiondecal "/Game/Art/Decals/M_SelectedEvilDecal.M_SelectedEvilDecal")))))

(fn `UserConstructionScript`
  (bind _returnvalue (`|GetDataTableRow` "/Game/Blueprints/Framework/Structs/DT_CharacterInfo.DT_CharacterInfo" (`self.RowID`))
    (:`then`
      (bind (_name _note _gameplaytags) (break `/Game/Blueprints/Framework/Structs/S_CharacterInfo` _returnvalue))
      (set `self.CharacterName` _name)
      (set `self.CharacterNote` _note)
      (set `self.GameplayTags` _gameplaytags)
      (`self.SetSelectedDecal`))))