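; Base actor for structures, configured from a data table and optionally able to hold an inventory.
; The construction script reads max health, inventory size and gameplay tags from DT_StructureInfo by row name, destroying the actor if no row matches.
; On BeginPlay, a non-zero inventory size adds an inventory system component at runtime with that size and a fixed interaction range.
; It exposes its gameplay tags, and LookAt returns empty text.
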(event `self.ReceiveBeginPlay`
  (if (!= (`self.InventorySize`) 0)
    (bind _returnvalue (`|AddComponentByClass` "/Game/Blueprints/Framework/Component/BPAC_InventorySystem.BPAC_InventorySystem_C"))
    (set `self.Ref_InventoryComponent` _returnvalue)
    (set `/Game/Blueprints/Framework/Component/BPAC_InventorySystem.InventorySize` (`self.InventorySize`) _returnvalue)
    (set `/Game/Blueprints/Framework/Component/BPAC_InventorySystem.InteractionRange` 300.0 _returnvalue)))

(fn `GetGameplayTags`
  (returns (Tags :type "GameplayTagContainer Structure"))
  (return (`self.GameplayTags`)))

(fn `LookAt`
  (returns (Message :type Text))
  (return ""))

(fn `UserConstructionScript`
  (bind _returnvalue (`|GetDataTableRow` "/Game/Blueprints/Framework/Structs/DT_StructureInfo.DT_StructureInfo" (`self.StructureID_RowName`))
    (:`then`
      (bind (_maxhealth _inventorysize _gameplaytags) (break `/Game/Blueprints/Framework/Structs/S_StructureInfo` _returnvalue))
      (set `self.MaxHealth` _maxhealth)
      (set `self.InventorySize` _inventorysize)
      (set `self.GameplayTags` _gameplaytags))
    (:`RowNotFound`
      (`self.K2_DestroyActor`))))