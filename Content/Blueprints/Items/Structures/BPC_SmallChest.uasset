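; Small chest structure that players interact with to open its inventory as a container.
; Interaction passes its inventory component to the FPS HUD's container display through the player controller.
; Cursor begin and end events report the chest's hover state to the top-down HUD.
; The construction script only runs the parent's setup.
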(event `/Game/Blueprints/Framework/Interfaces/BPI_Interacting.InteractWith`
  (params (PlayerCharacter :type "/Game/Blueprints/Player/BP_CharacterParent Object Reference"))
  (`/Game/Blueprints/UI/WB_FPS_Hud.ShowContainer` (`/Game/Blueprints/Framework/BP_PlayerController.Ref_FPS_HUD` (`/Game/Blueprints/Framework/BFL_GeneralUse.CastToPlayerController`)) (`self.Ref_InventoryComponent`)))

(event `self.ReceiveActorBeginCursorOver`
  (`/Game/Blueprints/UI/WB_TD_Hud.HoveredObjectUpdate` (`/Game/Blueprints/Framework/BP_PlayerController.Ref_TD_Hud` (`/Game/Blueprints/Framework/BFL_GeneralUse.CastToPlayerController`)) true self "None"))

(event `self.ReceiveActorEndCursorOver`
  (`/Game/Blueprints/UI/WB_TD_Hud.HoveredObjectUpdate` (`/Game/Blueprints/Framework/BP_PlayerController.Ref_TD_Hud` (`/Game/Blueprints/Framework/BFL_GeneralUse.CastToPlayerController`)) false self "None"))

(fn `UserConstructionScript`
  (`parent.UserConstructionScript`))