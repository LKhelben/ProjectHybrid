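; Parent Blueprint for item actors, identified by a row name in the DT_ItemInfo data table.
; The construction script fills the item data component with that row and a quantity of one, copies its gameplay tag, and destroys the actor if the row is missing.
; Cursor begin and end events report hover state and item ID to the player HUD.
; LookAt returns the item's table name, and GetGameplayTags exposes the copied tags.
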(event `self.ReceiveActorBeginCursorOver`
  (`/Game/Blueprints/UI/WB_TD_Hud.HoveredObjectUpdate` (`/Game/Blueprints/Framework/BP_PlayerController.Ref_TD_Hud` (`/Game/Blueprints/Framework/BFL_GeneralUse.CastToPlayerController`)) true self (`self.ItemID_RowName`)))

(event `self.ReceiveActorEndCursorOver`
  (`/Game/Blueprints/UI/WB_TD_Hud.HoveredObjectUpdate` (`/Game/Blueprints/Framework/BP_PlayerController.Ref_TD_Hud` (`/Game/Blueprints/Framework/BFL_GeneralUse.CastToPlayerController`)) false self "None"))

(fn `GetGameplayTags`
  (returns (Tags :type "GameplayTagContainer Structure"))
  (return (`self.GameplayTags`)))

(fn `LookAt`
  (returns (Message :type Text))
  (bind (_datatable _rowname) (break `DataTableRowHandle` (`/Game/Blueprints/Framework/Component/BPAC_ItemData.ItemID` (`self.BPAC_ItemData`))))
  (bind _returnvalue (`|GetDataTableRow` _datatable _rowname)
    (:`then`
      (return (`.Name_2_3B115EEE49661EC33CEC3D812843C4CC` (break `/Game/Blueprints/Framework/Structs/S_ItemInfo` _returnvalue))))))

(fn `UserConstructionScript`
  (bind _bpac_itemdata (`self.BPAC_ItemData`))
  (bind _itemid_rowname (`self.ItemID_RowName`))
  (bind _returnvalue (`|GetDataTableRow` "/Game/Blueprints/Framework/Structs/DT_ItemInfo.DT_ItemInfo" _itemid_rowname)
    (:`then`
      (set `/Game/Blueprints/Framework/Component/BPAC_ItemData.ItemID` (make `DataTableRowHandle` "/Game/Blueprints/Framework/Structs/DT_ItemInfo.DT_ItemInfo" _itemid_rowname) _bpac_itemdata)
      (set `/Game/Blueprints/Framework/Component/BPAC_ItemData.Quantity` 1 _bpac_itemdata)
      (set `self.GameplayTags` (`.GameplayTag_34_1E6A50204EEA3789D4EDEA94B3105ECB` (break `/Game/Blueprints/Framework/Structs/S_ItemInfo` _returnvalue))))
    (:`RowNotFound`
      (`self.K2_DestroyActor`))))