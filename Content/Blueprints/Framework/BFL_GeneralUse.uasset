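; BFL_GeneralUse is a Blueprint function library of shortcuts for reaching the local player's controller and character.
; Each function fetches the controller or character at player index 0 and returns it cast to a project class: BP_PlayerController, BP_CharacterParent for first-person, or BP_TopDownCharacter for top-down.
; A failed cast simply ends the function, with no fallback branch.
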(fn `CastToFPSPlayerCharacter`
  (returns (`AsBP Player Character` :type "/Game/Blueprints/Player/BP_CharacterParent Object Reference"))
  (bind _asbp_fpsplayer_character (cast `/Game/Blueprints/Player/BP_CharacterParent` (`GameplayStatics.GetPlayerCharacter` null)))
  (return _asbp_fpsplayer_character))

(fn `CastToPlayerController`
  (returns (`AsBP Player Controller` :type "/Game/Blueprints/Framework/BP_PlayerController Object Reference"))
  (bind _asbp_player_controller (cast `/Game/Blueprints/Framework/BP_PlayerController` (`GameplayStatics.GetPlayerController` null)))
  (return _asbp_player_controller))

(fn `CastToTDPlayerCharacter`
  (returns (`AsBP Top Down Character` :type "/Game/Blueprints/Player/BP_TopDownCharacter Object Reference"))
  (bind _asbp_top_down_character (cast `/Game/Blueprints/Player/BP_TopDownCharacter` (`GameplayStatics.GetPlayerCharacter` null)))
  (return _asbp_top_down_character))